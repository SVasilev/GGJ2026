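; Sheep actor that wanders, follows the player or flees, depending on proximity and the player's mask state.
; Pull and fear collision overlaps fire dispatchers: unmasked players attract it, masked players repel it.
; Mask changes arrive from the player's CmpPushPull component and re-trigger the matching behaviour.
; Delay loops reissue non-pathfinding AI MoveTo calls; random wandering around a saved origin resumes shortly after overlap ends outside fear range.
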(event OnComponentBeginOverlap(PulllColision)
  (params (OverlappedComponent :type Primitive%20Component%20Object%20Reference) (OtherActor :type Actor%20Object%20Reference) (OtherComp :type Primitive%20Component%20Object%20Reference) (OtherBodyIndex :type Integer) (bFromSweep :type Boolean) (SweepResult :type Hit%20Result%20Structure%20%28by%20ref%29))
  ;[0.15 0.15 0.15 0.5] Colision Checks
  (Utilities|Casting|CastToBP_TopDownCharacter OtherActor)
  (Variables|Default|SetbWithinPull true)
  (Default|CallMovetoPlayer))

(event OnComponentEndOverlap(PulllColision)
  (params (OverlappedComponent :type Primitive%20Component%20Object%20Reference) (OtherActor :type Actor%20Object%20Reference) (OtherComp :type Primitive%20Component%20Object%20Reference) (OtherBodyIndex :type Integer))
  ;[0.15 0.15 0.15 0.5] Colision Checks
  (Utilities|Casting|CastToBP_TopDownCharacter OtherActor)
  (Variables|Default|SetbWithinPull false)
  (Utilities|FlowControl|Delay 2.0)
  (if (not (Variables|Default|GetbWithinFear))
    (Default|CallStartWondering)))

(event OnComponentBeginOverlap(FearColision)
  (params (OverlappedComponent :type Primitive%20Component%20Object%20Reference) (OtherActor :type Actor%20Object%20Reference) (OtherComp :type Primitive%20Component%20Object%20Reference) (OtherBodyIndex :type Integer) (bFromSweep :type Boolean) (SweepResult :type Hit%20Result%20Structure%20%28by%20ref%29))
  ;[0.15 0.15 0.15 0.5] Colision Checks
  (Utilities|Casting|CastToBP_TopDownCharacter OtherActor)
  (Variables|Default|SetbWithinFear true)
  (Default|CallMoveAway))

(event OnComponentEndOverlap(FearColision)
  (params (OverlappedComponent :type Primitive%20Component%20Object%20Reference) (OtherActor :type Actor%20Object%20Reference) (OtherComp :type Primitive%20Component%20Object%20Reference) (OtherBodyIndex :type Integer))
  ;[0.15 0.15 0.15 0.5] Colision Checks
  (Utilities|Casting|CastToBP_TopDownCharacter OtherActor)
  (Variables|Default|SetbWithinFear false)
  (Utilities|FlowControl|Delay 2.0)
  (if (not (Variables|Default|GetbWithinFear))
    (Default|CallStartWondering)))

(event Custom|MoveToPlayer_Event
  ;[0.15 0.15 0.15 0.5] Pull Logic
  (Variables|Default|SetbIsWondering false)
  (if (not (Variables|Default|GetbHasMask))
    (AI|Navigation|MovetoLocation (AI|GetAIController self) (Transformation|GetActorLocation (Pawn|GetControlledPawn (Game|GetPlayerController 0))) -1.0 true false false true 0 :!label _label)
    (Utilities|FlowControl|Delay 0.1)
    (if (and (not (Variables|Default|GetbHasMask)) (Variables|Default|GetbWithinPull))
      (goto _label))))

(event Custom|StartWondering_Event
  ;[0.15 0.15 0.15 0.5] Wandering Behaviour
  (Variables|Default|SetbIsWondering true)
  (bind _output_get (Variables|Default|SetWondering%20Origin (Transformation|GetActorLocation self)))
  (AI|Navigation|MovetoLocation (AI|GetAIController self) (+ (* (* (Math|Random|RandomUnitVector) "1.000000,1.000000,0.000000") (Math|Conversions|ToVector(Float) 1.5e+02)) _output_get) -1.0 true false false true 0 :!label _label)
  (Utilities|FlowControl|Delay (Math|Random|RandomFloatinRange 1.0 2.5))
  (if (Variables|Default|GetbIsWondering)
    (goto _label)))

(event Custom|ChangeState_Event
  (params (bHasMask :type Boolean))
  ;[0.15 0.15 0.15 0.5] Change Mask From Player Behaviour
  (bind _output_get (Variables|Default|SetbHasMask bHasMask))
  (if _output_get
    (if (Variables|Default|GetbWithinFear)
      (Default|CallMoveAway))
    (elif (Variables|Default|GetbWithinPull)
      (Default|CallMovetoPlayer))))

(event Custom|MoveAway_Event
  (bind _self self)
  (bind _returnvalue (Transformation|GetActorLocation _self))
  ;[0.15 0.15 0.15 0.5] Push Logic
  (Variables|Default|SetbIsWondering false)
  (if (Variables|Default|GetbHasMask)
    (AI|Navigation|MovetoLocation (AI|GetAIController _self) (+ (- _returnvalue (Transformation|GetActorLocation (Pawn|GetControlledPawn (Game|GetPlayerController 0)))) _returnvalue) -1.0 true false false true 0 :!label _label)
    (Utilities|FlowControl|Delay 0.2)
    (if (and (Variables|Default|GetbHasMask) (Variables|Default|GetbWithinFear))
      (goto _label))))

(event EventBeginPlay
  ;[0.15 0.15 0.15 0.5] BeginPlay
  (EventDispatchers|AssignMovetoPlayer (EventDispatchers|CreateEvent :!event Custom|MoveToPlayer_Event))
  (bind _asbp_top_down_character (Utilities|Casting|CastToBP_TopDownCharacter (Pawn|GetControlledPawn (Game|GetPlayerController 0))))
  (EventDispatchers|AssignChangeState (Variables|/Game/GGJ2026/Game/Blueprints/BP_TopDownCharacter.BP_TopDownCharacter_C|GetCmp_PushPull _asbp_top_down_character) (EventDispatchers|CreateEvent :!event Custom|ChangeState_Event))
  (EventDispatchers|BindEventtoMoveAway (EventDispatchers|CreateEvent :!event Custom|MoveAway_Event))
  (EventDispatchers|BindEventtoStartWondering (EventDispatchers|CreateEvent :!event Custom|StartWondering_Event))
  (Default|CallStartWondering))

(fn ConstructionScript)