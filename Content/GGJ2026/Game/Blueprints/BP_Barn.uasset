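; BP_Barn is the barn actor that takes in sheep and counts each one only once.
; When a sheep's capsule enters its box, the barn registers it, stops its AI movement and sends it toward an interior target, repeating the move after a short delay.
; It also shrinks the capsule, enables movement avoidance, flags the sheep as in the barn and fires a SheepEnteredBarn event.
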(event OnComponentBeginOverlap(Box)
  (params (OverlappedComponent :type Primitive%20Component%20Object%20Reference) (OtherActor :type Actor%20Object%20Reference) (OtherComp :type Primitive%20Component%20Object%20Reference) (OtherBodyIndex :type Integer) (bFromSweep :type Boolean) (SweepResult :type Hit%20Result%20Structure%20%28by%20ref%29))
  (Utilities|Casting|CastToCapsuleComponent OtherComp)
  (bind _asbp_sheep (Utilities|Casting|CastToBP_Sheep OtherActor))
  (if (not (Utilities|Array|ContainsItem (Variables|Default|GetRegisteredSheep) _asbp_sheep))
    (Utilities|Array|Add (Variables|Default|GetRegisteredSheep) _asbp_sheep)
    (AI|Navigation|StopMovement (AI|GetAIController _asbp_sheep))
    ;[0.15 0.15 0.15 0.5 14] Makes the Sheep circle around in the Barn. Maybe we want to resort back to basic Patrolling and DIsable Collisions
    (AI|Navigation|SimpleMovetoLocation (AI|GetAIController _asbp_sheep) (Transformation|GetWorldLocation (Variables|Default|GetTarget)))
    (Components|Capsule|SetCapsuleRadius (Variables|/Script/Engine.Character|GetCapsuleComponent _asbp_sheep) 1e+01 true)
    (Class|CharacterMovementComponent|SetAvoidanceEnabled (Variables|/Script/Engine.Character|GetCharacterMovement _asbp_sheep) true)
    (Variables|/Game/GGJ2026/Game/Blueprints/BP_Sheep.BP_Sheep_C|SetbIsInBarn _asbp_sheep true)
    (Utilities|FlowControl|Sequence
      (:then_0
        (Utilities|FlowControl|Delay 2.6)
        (AI|Navigation|SimpleMovetoLocation (AI|GetAIController _asbp_sheep) (Transformation|GetWorldLocation (Variables|Default|GetTarget))))
      (:then_1
        (Default|CallSheepEnteredBarn)))))

(fn ConstructionScript)